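; BP_AlertTaskSpawner spawns alert task actors at its own transform in the SpaceBus game mode until the game ends.
; In the alternate mode, a looping timer spawns every minute, then switches the class from light switch to pressure plate manager; the reverse branch assigns the failed cast result.
; Otherwise it spawns once, either on game start or at a random time in the round's second half.
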(event `self.ReceiveBeginPlay`
  ; Event BeginPlay
  (bind _cachedgamemode (`self.GetAndCacheGM_SpaceBus`))
  (if (`self.alternateGameMode`)
    ;; Spawn an alert task every 60 seconds if the game is not over
    (`KismetSystemLibrary.K2_SetTimerDelegate` (delegate `Spawn Alert Task`) 60.0 true)
    (elif (`self.spawnInSecondHalfOfRound`)
      (bind _roundtime (`/Game/Blueprints/GameModes/GM_SpaceBus.roundTime` _cachedgamemode))
      (`KismetSystemLibrary.K2_SetTimerDelegate` (delegate `Spawn Actor at Location`) (`KismetMathLibrary.RandomFloatInRange` (* _roundtime 0.5) (* _roundtime 0.75)))
      (else
        (add `/Game/Blueprints/GameModes/GM_SpaceBus.On Game Started` (`self.cachedGameMode`) (delegate `Spawn Actor at Location`))))))

(event `Spawn Actor at Location`
  (bind _actor_to_spawn (`self.Actor to Spawn`))
  ; Event BeginPlay
  (if (not (`/Game/Blueprints/GameModes/GM_SpaceBus.isGameOver?` (`self.cachedGameMode`)))
    (if (`KismetSystemLibrary.IsValidClass` _actor_to_spawn)
      (`|SpawnActorFromClass` _actor_to_spawn (`SceneComponent.K2_GetComponentToWorld` (`self.DefaultSceneRoot`)) "Undefined" "MultiplyWithRoot" null null))))

(event `Spawn Alert Task`
  (bind _actor_to_spawn (`self.Actor to Spawn`))
  ; Event BeginPlay
  ;; Spawn an alert task every 60 seconds if the game is not over
  (if (not (`/Game/Blueprints/GameModes/GM_SpaceBus.isGameOver?` (`self.cachedGameMode`)))
    ;;; Spawn alert task child class from variable at world location
    (if (`KismetSystemLibrary.IsValidClass` _actor_to_spawn)
      (`|SpawnActorFromClass` _actor_to_spawn (`SceneComponent.K2_GetComponentToWorld` (`self.DefaultSceneRoot`)) "Undefined" "MultiplyWithRoot" null null)
      ;;; Swap class variable to alternate between child classes
      (bind _asbp_light_switch_manager (castclass `/Game/Blueprints/Tasks/BP_LightSwitchManager` (`self.Actor to Spawn`))
        (:`then`
          (set `self.Actor to Spawn` "/Game/Blueprints/Tasks/BP_PressurePlateManager.BP_PressurePlateManager_C"))
        (:`CastFailed`
          (set `self.Actor to Spawn` _asbp_light_switch_manager))))))

(fn `GetAndCacheGM_SpaceBus`
  (returns (CachedGameMode :type "/Game/Blueprints/GameModes/GM_SpaceBus Object Reference"))
  (bind _asgm_space_bus (cast `/Game/Blueprints/GameModes/GM_SpaceBus` (`GameplayStatics.GetGameMode`)))
  (bind _output_get (set `self.cachedGameMode` _asgm_space_bus))
  (return _output_get))

(fn `UserConstructionScript`)