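; Engine repair task, a child of a shared task Blueprint, that restores ship health when the player completes it with the required item.
; Completion adds health and updates the UI, destroying the task only if the increase fits within starting health.
; In alternate game mode it instead applies a capped cryopod health change when the player collision check returns false, then destroys itself.
; Box overlap shows the button prompt to wrench holders; failure destroys the actor.
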(event `self.ReceiveBeginPlay`
  (`parent.ReceiveBeginPlay`))

(event `self.ReceiveTick`
  (params (DeltaSeconds :type "Float (single-precision)"))
  (`parent.ReceiveTick` DeltaSeconds))

(event `self.TaskFailed`
  (`self.K2_DestroyActor`))

(event `/Game/Blueprints/Interfaces/BPI_UseItem.Complete Task`
  (bind _cryopod (`self.cryopod`))
  (bind _shiphealthincrease (`self.shipHealthIncrease`))
  (bind _cachedgamemode (`self.cachedGameMode`))
  (bind _shiphealth (`/Game/Blueprints/GameModes/GM_SpaceBus.shipHealth` _cachedgamemode))
  ; Override Task Completed Logic to increase ship health when completed
  (bind _result (`self.checkPlayerItem`))
  (if (`self.alternateGameMode`)
    (bind _hit_result (`self.checkCollisionBetweenPlayerAndSelf`))
    (if (not _hit_result)
      (`FMODBlueprintStatics.PlayEvent2D` "/Game/FMOD/Events/SFX/SFX_-_Engine_Repair_Sound.SFX_-_Engine_Repair_Sound")
      (if (not (> (- (`/Game/Blueprints/LevelBlueprints/BP_Cryopod.cryoPodHealth` _cryopod) (`self.cryopodDamage`)) (`/Game/Blueprints/LevelBlueprints/BP_Cryopod.initialCryoPodHealth` _cryopod)))
        (`/Game/Blueprints/LevelBlueprints/BP_Cryopod.damageCryopod` _cryopod (`self.cryopodDamage`)))
      (`self.K2_DestroyActor`))
    (elif _result
      (`GameplayStatics.SpawnSound2D` "/Game/Audio/In-House/SW_TaskComplete.SW_TaskComplete" 1.0 1.0 0.0 null)
      ;; Check if health is low enough for increase
      (if (<= _shiphealth (- (`/Game/Blueprints/GameModes/GM_SpaceBus.startingShipHealth` _cachedgamemode) _shiphealthincrease))
        (bind _output_get (set `/Game/Blueprints/GameModes/GM_SpaceBus.shipHealth` (+ _shiphealth _shiphealthincrease) _cachedgamemode))
        (`/Game/UI/WidgetBlueprints/WBP_UI.UpdateShipHealth` (`/Game/Blueprints/GameModes/GM_SpaceBus.UserInterface` _cachedgamemode) _output_get)
        (`self.K2_DestroyActor`)))))

(event `self.Box Collision.OnComponentBeginOverlap`
  (params (OverlappedComponent :type "PrimitiveComponent Object Reference") (OtherActor :type "Actor Object Reference") (OtherComp :type "PrimitiveComponent Object Reference") (OtherBodyIndex :type Integer) (bFromSweep :type Boolean) (SweepResult :type "HitResult Structure (by ref)"))
  (bind _interactingplayer (`self.interactingPlayer`))
  (`self.playerEnters` OtherActor)
  (`/Engine/EditorBlueprintResources/StandardMacros.IsValid` _interactingplayer
    (:`Is Valid`
      (if (`/Game/Blueprints/Characters/BP_ThirdPersonCharacter.HasWrench` _interactingplayer)
        (`SceneComponent.SetHiddenInGame` (`self.ButtonPromptWidgetComponent`) false false)))))

(event `self.Box Collision.OnComponentEndOverlap`
  (params (OverlappedComponent :type "PrimitiveComponent Object Reference") (OtherActor :type "Actor Object Reference") (OtherComp :type "PrimitiveComponent Object Reference") (OtherBodyIndex :type Integer))
  (`self.playerExits` OtherActor))

(fn `UserConstructionScript`
  (`parent.UserConstructionScript`))