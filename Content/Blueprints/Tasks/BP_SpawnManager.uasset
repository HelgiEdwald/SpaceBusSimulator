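; Task spawn manager that, while active, populates a level with recurring tasks through an array of spawners.
; After the SpaceBus game mode's countdown, it shuffles the spawners and triggers a starting batch with random delays.
; A looping timer, its interval randomized once at BeginPlay, spawns at a random available spawner until game over.
; The Cryopod's pseudo-destroyed event deactivates the manager and clears that timer.
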(event `self.ReceiveBeginPlay`
  ; Event Begin Play
  (if (`self.isActive`)
    (bind _cachedgamemode (`self.GetAndCacheGM_SpaceBus`))
    ;; Spawn tasks after countdown
    (`KismetSystemLibrary.K2_SetTimerDelegate` (delegate `SpawnStartingRecurringTasks`) (`KismetMathLibrary.Conv_IntToDouble` (`/Game/Blueprints/GameModes/GM_SpaceBus.Countdown Time` _cachedgamemode)))
    ;; Check at an interval if there is an available spawner and spawn if available
    (bind _returnvalue (`KismetSystemLibrary.K2_SetTimerDelegate` (delegate `Spawn New Task`) (`KismetMathLibrary.RandomFloatInRange` (`self.SpawnMin`) (`self.SpawnMax`)) true false 10.0))
    (set `self.spawnTimerHandle` _returnvalue)
    (add `/Game/Blueprints/LevelBlueprints/BP_Cryopod.OnPseudoDestroyed` (`self.cryopod`) (delegate `disableSpawner`))))

(event `disableSpawner`
  ; Event Begin Play
  ;; Check at an interval if there is an available spawner and spawn if available
  (set `self.isActive` false)
  (`KismetSystemLibrary.K2_ClearAndInvalidateTimerHandle` (`self.spawnTimerHandle`)))

(event `Spawn New Task`
  (bind _spawnerarray (`self.spawnerArray`))
  ; Event Begin Play
  ;; Check at an interval if there is an available spawner and spawn if available
  (if (not (`/Game/Blueprints/GameModes/GM_SpaceBus.isGameOver?` (`self.cachedGameMode`)))
    (`KismetArrayLibrary.Array_Shuffle` _spawnerarray)
    (for _array_element _spawnerarray
      (bind _spawneravailable (`/Game/Blueprints/Tasks/BP_RecurringTaskSpawner.spawnerAvailable` _array_element))
      (if _spawneravailable
        (set `self.foundAvailableSpawn` _spawneravailable)
        (`/Game/Blueprints/Tasks/BP_RecurringTaskSpawner.Spawn Actor at Location` _array_element)
        (break)))))

(event `SpawnStartingRecurringTasks`
  (bind _spawnerarray (`self.spawnerArray`))
  ; Event Begin Play
  ;; Spawn tasks after countdown
  ;;; Shuffle array and spawn based on starting number
  (`KismetSystemLibrary.Delay` (`KismetMathLibrary.RandomFloatInRange` (`self.initSpawnMin`) (`self.initSpawnMax`)))
  (`KismetArrayLibrary.Array_Shuffle` _spawnerarray)
  (for (_array_element _array_index) _spawnerarray
    (if (not (== _array_index (`self.numStartingTasks`)))
      (`/Game/Blueprints/Tasks/BP_RecurringTaskSpawner.Spawn Actor at Location` _array_element)
      (set `/Game/Blueprints/Tasks/BP_RecurringTaskSpawner.spawnerAvailable` false _array_element)
      (`KismetSystemLibrary.Delay` (`KismetMathLibrary.RandomFloatInRange` (`self.initSpawnMin`) (`self.initSpawnMax`)))
      (else
        (break)))))

(fn `GetAndCacheGM_SpaceBus`
  (returns (CachedGameMode :type "/Game/Blueprints/GameModes/GM_SpaceBus Object Reference"))
  (bind _asgm_space_bus (cast `/Game/Blueprints/GameModes/GM_SpaceBus` (`GameplayStatics.GetGameMode`)))
  (bind _output_get (set `self.cachedGameMode` _asgm_space_bus))
  (return _output_get))

(fn `UserConstructionScript`)