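; Spawner for recurring tasks in the SpaceBus game mode, creating a random task actor at its own transform and linking it to a cryopod.
; SpawnActoratLocation skips spawning once the game is over or without a valid cryopod.
; It marks itself unavailable after spawning, then available again shortly after the task is destroyed.
; The repair engine task joins the random pool at BeginPlay or, optionally, halfway through the round.
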(event `AddRepairEngineTask`
  ; In later half of round, add repair engine task to possible spawn array
  (`KismetArrayLibrary.Array_Add` (`self.recurringTaskClassessArray`) "/Game/Blueprints/Tasks/BP_RepairEngineTask.BP_RepairEngineTask_C"))

(event `self.ReceiveBeginPlay`
  (bind _cachedgamemode (`self.cachedGameMode`))
  (`self.GetAndCacheGM_SpaceBus`)
  (if (`self.addRepairEngineLater`)
    ; In later half of round, add repair engine task to possible spawn array
    (`KismetSystemLibrary.K2_SetTimerDelegate` (delegate `AddRepairEngineTask`) (`KismetMathLibrary.Conv_IntToDouble` (+ (`/Game/Blueprints/GameModes/GM_SpaceBus.Countdown Time` _cachedgamemode) (* (`/Game/Blueprints/GameModes/GM_SpaceBus.roundTime` _cachedgamemode) 0.5))))
    (else
      (`KismetArrayLibrary.Array_Add` (`self.recurringTaskClassessArray`) "/Game/Blueprints/Tasks/BP_RepairEngineTask.BP_RepairEngineTask_C"))))

(event `Spawn Actor at Location`
  (`self.randomiseAndSetTaskToSpawn`)
  ; Check if game over
  (if (not (`/Game/Blueprints/GameModes/GM_SpaceBus.isGameOver?` (`self.cachedGameMode`)))
    ; Spawn Actor at Transform
    (`/Engine/EditorBlueprintResources/StandardMacros.IsValid` (`self.cryopod`)
      (:`Is Valid`
        (bind _returnvalue (`|SpawnActorFromClass` (`self.Actor to Spawn`) (`SceneComponent.K2_GetComponentToWorld` (`self.DefaultSceneRoot`)) "Undefined" "MultiplyWithRoot" null null))
        (`/Game/Blueprints/Tasks/BP_RecurringTask.initCryopod` _returnvalue (`self.cryopod`))
        ; Mark spawner as unavailable after spawning and as available when spawned actor is destroyed
        (set `self.spawnerAvailable` false)
        (add `/Game/Blueprints/Tasks/BP_RecurringTask.OnIHaveBeenDestroyed` _returnvalue (delegate `HandleDestruction`))))))

(event `HandleDestruction`
  ; Mark spawner as unavailable after spawning and as available when spawned actor is destroyed
  (`KismetSystemLibrary.K2_SetTimerDelegate` (delegate `SpawnAvailable`) 5.0))

(event `SpawnAvailable`
  ; Mark spawner as unavailable after spawning and as available when spawned actor is destroyed
  (set `self.spawnerAvailable` true))

(fn `GetAndCacheGM_SpaceBus`
  (returns (CachedGameMode :type "/Game/Blueprints/GameModes/GM_SpaceBus Object Reference"))
  (bind _asgm_space_bus (cast `/Game/Blueprints/GameModes/GM_SpaceBus` (`GameplayStatics.GetGameMode`)))
  (bind _output_get (set `self.cachedGameMode` _asgm_space_bus))
  (return _output_get))

(fn `randomiseAndSetTaskToSpawn`
  (set `self.Actor to Spawn` (`KismetArrayLibrary.Array_Random` (`self.recurringTaskClassessArray`))))

(fn `UserConstructionScript`)