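; Timed alert task actor that plays a cue and shows a countdown widget on BeginPlay.
; A one-shot timer triggers failure, while a separate looping timer updates the displayed time only during active play.
; Failure fires OnAlertTaskFailed, destroys the actor, then damages tagged cryopods in alternate mode or cuts GM_SpaceBus ship health, possibly ending the game.
; Completion plays a sound, clears the failure timer and removes the widget.
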(event `self.ReceiveBeginPlay`
  (bind _alertwidget (`self.alertWidget`))
  (`GameplayStatics.PlaySound2D` "/Game/Audio/In-House/SW_AlertTaskCue.SW_AlertTaskCue" 1.0 1.0 0.0 null null)
  ; Get and set variable values at start-up
  (`self.GetAndCacheGM_SpaceBus`)
  (`self.createUI`)
  (`/Game/UI/WidgetBlueprints/WBP_AlertTaskActive.UpdateTime` _alertwidget (`self.timeToFailure`))
  (`/Game/UI/WidgetBlueprints/WBP_AlertTaskActive.changeDescription` _alertwidget (`self.alertTaskText`))
  ; Start a timer, fail alert task when timer expires
  (bind _returnvalue (`KismetSystemLibrary.K2_SetTimerDelegate` (delegate `alertTaskNotCompletedInTime`) (`self.timeToFailure`)))
  (set `self.alertTaskRunOutTimer` _returnvalue)
  ; Update UI every second if the game is not over, manually track time left
  (`KismetSystemLibrary.K2_SetTimerDelegate` (delegate `DecreaseTimer`) 1.0 true))

(event `alertTaskNotCompletedInTime`
  ; Start a timer, fail alert task when timer expires
  (`self.AlertTaskFailed`))

(event `DecreaseTimer`
  (bind _cachedgamemode (`self.cachedGameMode`))
  ; Update UI every second if the game is not over, manually track time left
  (if (`/Game/Blueprints/GameModes/GM_SpaceBus.gameStarted` _cachedgamemode)
    (if (not (`/Game/Blueprints/GameModes/GM_SpaceBus.isGameOver?` _cachedgamemode))
      (bind _result (`/Engine/EditorBlueprintResources/StandardMacros.DecrementFloat` (`self.timeToFailure`))
        (:`  `
          (`/Game/UI/WidgetBlueprints/WBP_AlertTaskActive.UpdateTime` (`self.alertWidget`) _result))))))

(fn `AlertTaskCompleted`
  (`GameplayStatics.PlaySound2D` "/Game/Audio/In-House/SW_AlertTaskComplete.SW_AlertTaskComplete" 1.0 1.0 0.0 null null)
  (`KismetSystemLibrary.K2_ClearAndInvalidateTimerHandle` (`self.alertTaskRunOutTimer`))
  (`self.deleteUI`))

(fn `AlertTaskFailed`
  (bind _cachedgamemode (`self.cachedGameMode`))
  (bind _cachedgamemode_2 (`self.cachedGameMode`))
  (`self.OnAlertTaskFailed`)
  (`GameplayStatics.PlaySound2D` "/Game/Audio/In-House/SW_AlertTaskFailed.SW_AlertTaskFailed" 1.0 1.0 0.0 null null)
  (`self.K2_DestroyActor`)
  (`self.deleteUI`)
  (if (`self.alternateGameMode`)
    (bind _outactors (`GameplayStatics.GetAllActorsWithTag` "Cryopod"))
    (for _array_element _outactors
      (bind _asbp_cryopod (cast `/Game/Blueprints/LevelBlueprints/BP_Cryopod` _array_element))
      (`/Game/Blueprints/LevelBlueprints/BP_Cryopod.damageCryopod` _asbp_cryopod (`self.cryopodDamage`)))
    (elif (not (`/Game/Blueprints/GameModes/GM_SpaceBus.isGameOver?` _cachedgamemode))
      (bind _output_get (set `/Game/Blueprints/GameModes/GM_SpaceBus.shipHealth` (- (`/Game/Blueprints/GameModes/GM_SpaceBus.shipHealth` _cachedgamemode) (* (`/Game/Blueprints/GameModes/GM_SpaceBus.startingShipHealth` _cachedgamemode) 0.3)) _cachedgamemode))
      (`/Game/UI/WidgetBlueprints/WBP_UI.UpdateShipHealth` (`/Game/Blueprints/GameModes/GM_SpaceBus.UserInterface` _cachedgamemode) _output_get)
      (if (<= (`/Game/Blueprints/GameModes/GM_SpaceBus.shipHealth` _cachedgamemode_2) 0.0)
        (`/Game/Blueprints/GameModes/GM_SpaceBus.ShowEndScreen` _cachedgamemode_2 false)))))

(fn `createUI`
  (bind _returnvalue (`|CreateWidget` "/Game/UI/WidgetBlueprints/WBP_AlertTaskActive.WBP_AlertTaskActive_C"))
  (set `self.alertWidget` _returnvalue)
  (`UserWidget.AddToViewport` _returnvalue 0)
  (`UserWidget.AddToViewport` (`/Game/Blueprints/GameModes/GM_SpaceBus.UserInterface` (`self.cachedGameMode`)) 0))

(fn `deleteUI`
  (`Widget.RemoveFromParent` (`self.alertWidget`)))

(fn `GetAndCacheGM_SpaceBus`
  (returns (CachedGameMode :type "/Game/Blueprints/GameModes/GM_SpaceBus Object Reference"))
  (bind _asgm_space_bus (cast `/Game/Blueprints/GameModes/GM_SpaceBus` (`GameplayStatics.GetGameMode`)))
  (bind _output_get (set `self.cachedGameMode` _asgm_space_bus))
  (return _output_get))

(fn `UserConstructionScript`)