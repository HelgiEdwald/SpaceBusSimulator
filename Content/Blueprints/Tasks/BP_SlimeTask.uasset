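; BP_SlimeTask is a slime task that shows a button prompt when a player carrying a broom enters its trigger box.
; Box collision overlaps pass the actor to PlayerEnters and PlayerExits, and the prompt is unhidden only if InteractingPlayer is then valid and has HasBroom set.
; BeginPlay, Tick and construction only call the parent, and this graph never hides the prompt itself.
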(event `self.ReceiveBeginPlay`
  (`parent.ReceiveBeginPlay`))

(event `self.ReceiveTick`
  (params (DeltaSeconds :type "Float (single-precision)"))
  (`parent.ReceiveTick` DeltaSeconds))

(event `self.Box Collision.OnComponentBeginOverlap`
  (params (OverlappedComponent :type "PrimitiveComponent Object Reference") (OtherActor :type "Actor Object Reference") (OtherComp :type "PrimitiveComponent Object Reference") (OtherBodyIndex :type Integer) (bFromSweep :type Boolean) (SweepResult :type "HitResult Structure (by ref)"))
  (bind _interactingplayer (`self.interactingPlayer`))
  (`self.playerEnters` OtherActor)
  (`/Engine/EditorBlueprintResources/StandardMacros.IsValid` _interactingplayer
    (:`Is Valid`
      (if (`/Game/Blueprints/Characters/BP_ThirdPersonCharacter.HasBroom` _interactingplayer)
        (`SceneComponent.SetHiddenInGame` (`self.ButtonPromptWidgetComponent`) false false)))))

(event `self.Box Collision.OnComponentEndOverlap`
  (params (OverlappedComponent :type "PrimitiveComponent Object Reference") (OtherActor :type "Actor Object Reference") (OtherComp :type "PrimitiveComponent Object Reference") (OtherBodyIndex :type Integer))
  (`self.playerExits` OtherActor))

(fn `UserConstructionScript`
  (`parent.UserConstructionScript`))