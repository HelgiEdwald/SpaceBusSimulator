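; Base item actor that offers itself to one nearby player at a time, highlighting and showing a button prompt.
; Box overlap with a PlayerCylinder-tagged component claims the item for an empty-handed character not already in a box, setting its NearbyItem and enabling custom depth.
; End overlap by that player releases it.
; The prompt's texture is set on BeginPlay, and Tick tilts it toward the camera with yaw fixed.
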(event `self.ReceiveBeginPlay`
  (`self.setButtonImage` (`self.buttonImage`) (`self.ButtonWidget`)))

(event `self.ReceiveTick`
  (params (DeltaSeconds :type "Float (single-precision)"))
  (`self.rotateWidgetTowardsCamera` (`self.ButtonWidget`)))

(event `self.Box Collision.OnComponentBeginOverlap`
  (params (OverlappedComponent :type "PrimitiveComponent Object Reference") (OtherActor :type "Actor Object Reference") (OtherComp :type "PrimitiveComponent Object Reference") (OtherBodyIndex :type Integer) (bFromSweep :type Boolean) (SweepResult :type "HitResult Structure (by ref)"))
  (if (`ActorComponent.ComponentHasTag` OtherComp "PlayerCylinder")
    (bind _asbp_third_person_character (cast `/Game/Blueprints/Characters/BP_ThirdPersonCharacter` OtherActor))
    (if (not (`/Game/Blueprints/Characters/BP_ThirdPersonCharacter.isInBoundingBox` _asbp_third_person_character))
      (set `/Game/Blueprints/Characters/BP_ThirdPersonCharacter.isInBoundingBox` true _asbp_third_person_character)
      (if (not (`/Game/Blueprints/Characters/BP_ThirdPersonCharacter.HasItem` _asbp_third_person_character))
        (if (`self.isAvailable`)
          (set `self.isAvailable` false)
          (set `self.interactingPlayer` _asbp_third_person_character)
          (`PrimitiveComponent.SetRenderCustomDepth` (`self.ITEM`) true)
          (`SceneComponent.SetHiddenInGame` (`self.ButtonWidget`) false false)
          (set `/Game/Blueprints/Characters/BP_ThirdPersonCharacter.nearItem` true _asbp_third_person_character)
          (set `/Game/Blueprints/Characters/BP_ThirdPersonCharacter.nearbyItem` self _asbp_third_person_character))))))

(event `self.Box Collision.OnComponentEndOverlap`
  (params (OverlappedComponent :type "PrimitiveComponent Object Reference") (OtherActor :type "Actor Object Reference") (OtherComp :type "PrimitiveComponent Object Reference") (OtherBodyIndex :type Integer))
  (bind _interactingplayer (`self.interactingPlayer`))
  (if (`ActorComponent.ComponentHasTag` OtherComp "PlayerCylinder")
    (`/Engine/EditorBlueprintResources/StandardMacros.IsValid` _interactingplayer
      (:`Is Valid`
        (if (== _interactingplayer OtherActor)
          (set `/Game/Blueprints/Characters/BP_ThirdPersonCharacter.nearItem` false _interactingplayer)
          (set `/Game/Blueprints/Characters/BP_ThirdPersonCharacter.nearbyItem` null _interactingplayer)
          (set `/Game/Blueprints/Characters/BP_ThirdPersonCharacter.isInBoundingBox` false _interactingplayer)
          (set `self.interactingPlayer` null)
          (set `self.isAvailable` true)
          (`SceneComponent.SetHiddenInGame` (`self.ButtonWidget`) true false)
          (`PrimitiveComponent.SetRenderCustomDepth` (`self.ITEM`) false))))))

(fn `rotateWidgetTowardsCamera`
  (params (`Widget Component` :type "WidgetComponent Object Reference"))
  (bind (_returnvalue_roll _returnvalue_pitch) (`KismetMathLibrary.BreakRotator` (`KismetMathLibrary.FindLookAtRotation` (`SceneComponent.K2_GetComponentLocation` `Widget Component`) (`SceneComponent.K2_GetComponentLocation` (`PlayerCameraManager.TransformComponent` (`UserWidget.GetOwningPlayerCameraManager` (`WidgetComponent.GetUserWidgetObject` `Widget Component`)))))))
  (`SceneComponent.K2_SetWorldRotation` `Widget Component` (`KismetMathLibrary.MakeRotator` (+ _returnvalue_roll 180.0) (+ _returnvalue_pitch 90.0)) false false))

(fn `setButtonImage`
  (params (textureToUse :type "Texture2D Object Reference") (widgetComponent :type "WidgetComponent Object Reference"))
  (bind _aswbp_button_prompt (cast `/Game/UI/WidgetBlueprints/WBP_ButtonPrompt` (`WidgetComponent.GetUserWidgetObject` widgetComponent)))
  (set `/Game/UI/WidgetBlueprints/WBP_ButtonPrompt.buttonTexture` textureToUse _aswbp_button_prompt))

(fn `UserConstructionScript`)