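; Pickup item actor that gives the third-person character an equippable item and then removes itself from the world.
; Box collision overlaps toggle whether it can be picked up, and the construction script applies a configurable mesh.
; PickUp waits a tick, then flags overlapping characters as holding an item and sets their EquippedItem child actor class.
; It marks itself picked up even when out of range, and Tick destroys it.
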(event `/Game/Blueprints/Interfaces/BPI_PickUpItems.PickUp`
  (`KismetSystemLibrary.PrintString` "Player Picked Up Water Jug")
  (`KismetSystemLibrary.DelayUntilNextTick`)
  (set `self.ItemPickedUp` true)
  (for _array_element (`PrimitiveComponent.GetOverlappingActors` (`self.Box Collision`) "/Game/Blueprints/Characters/BP_ThirdPersonCharacter.BP_ThirdPersonCharacter_C")
    (if (`self.ItemCanBePickedUp`)
      (bind _asbp_third_person_character (cast `/Game/Blueprints/Characters/BP_ThirdPersonCharacter` _array_element))
      (set `/Game/Blueprints/Characters/BP_ThirdPersonCharacter.HasItem` true _asbp_third_person_character)
      (`ChildActorComponent.SetChildActorClass` (`/Game/Blueprints/Characters/BP_ThirdPersonCharacter.EquippedItem` _asbp_third_person_character) (`self.In Class`))
      (set `self.ItemPickedUp` true))))

(event `self.Box Collision.OnComponentBeginOverlap`
  (params (OverlappedComponent :type "PrimitiveComponent Object Reference") (OtherActor :type "Actor Object Reference") (OtherComp :type "PrimitiveComponent Object Reference") (OtherBodyIndex :type Integer) (bFromSweep :type Boolean) (SweepResult :type "HitResult Structure (by ref)"))
  ; Is the player close enough to pick up the item?
  (set `self.ItemCanBePickedUp` true))

(event `self.ReceiveTick`
  (params (DeltaSeconds :type "Float (single-precision)"))
  (if (`self.ItemPickedUp`)
    (`self.K2_DestroyActor`)))

(event `self.Box Collision.OnComponentEndOverlap`
  (params (OverlappedComponent :type "PrimitiveComponent Object Reference") (OtherActor :type "Actor Object Reference") (OtherComp :type "PrimitiveComponent Object Reference") (OtherBodyIndex :type Integer))
  ; Is the player close enough to pick up the item?
  (set `self.ItemCanBePickedUp` false))

(fn `UserConstructionScript`
  (`StaticMeshComponent.SetStaticMesh` (`self.Sphere`) (`self.Pick Up Item`)))