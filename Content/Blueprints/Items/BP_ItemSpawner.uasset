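; Item spawner actor that spawns one configurable item class at its own position when play begins.
; BeginPlay passes ItemToSpawn to SpawnItem, which spawns the actor at the root component's relative location and clears IsAvailable.
; The ItemGrabbed event sets IsAvailable back to true but triggers no respawn, and nothing in this Blueprint reads the flag.
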(event `/Game/Blueprints/Interfaces/BPI_ItemGrabbed.itemGrabbed`
  (set `self.isAvailable` true))

(event `self.ReceiveBeginPlay`
  (`self.SpawnItem` (`self.itemToSpawn`)))

(fn `SpawnItem`
  (params (Class :type "Actor Class Reference"))
  (`|SpawnActorFromClass` Class (`KismetMathLibrary.Conv_VectorToTransform` (`SceneComponent.RelativeLocation` (`self.DefaultSceneRoot`))) "Undefined" "MultiplyWithRoot" null null)
  (set `self.isAvailable` false))

(fn `UserConstructionScript`)