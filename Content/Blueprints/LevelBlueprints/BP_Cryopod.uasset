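; Per-player cryopod in the SpaceBus game mode, acting as that player's life with a camera-facing health bar widget.
; DamageCryopod updates the bar and game-mode leaderboard, swaps to a damaged mesh, and destroys the owning player at zero health.
; It then counts living pods: with two or more left it shows the destroyed mesh and mutes that player's music track via a global audio parameter, otherwise it triggers the end screen.
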(event `self.ReceiveBeginPlay`
  (bind _returnvalue (`KismetStringLibrary.Conv_StringToName` (`KismetStringLibrary.Concat_StrStr` "player" (`KismetStringLibrary.Conv_IntToString` (`self.playerNumber`)) "track")))
  (bind _returnvalue_2 (`FMODBlueprintStatics.GetGlobalParameterByName` _returnvalue))
  (set `self.playerTrackName` _returnvalue)
  (`PrimitiveComponent.SetMaterial` (`self.Pod`) 0 (`self.podShellMaterial`))
  ; get and cache ui and other cryopods
  (`PrimitiveComponent.SetMaterial` (`self.Base`) 1 (`self.baseMaterial`))
  (bind _aswbp_cryopod_health (cast `/Game/UI/WidgetBlueprints/WBP_CryopodHealth` (`WidgetComponent.GetUserWidgetObject` (`self.Widget`))))
  (set `self.cachedWBPClassObject` _aswbp_cryopod_health)
  (bind _outactors (`GameplayStatics.GetAllActorsOfClass` "BP_Cryopod_C"))
  (set `self.allCryopods` _outactors))

(event `self.ReceiveTick`
  (params (DeltaSeconds :type "Float (single-precision)"))
  (`self.rotateWidgetTowardsCamera` (`self.Widget`)))

(fn `damageCryopod`
  (params (damage :type "Float (double-precision)"))
  (bind _owningplayer (`self.owningPlayer`))
  ; Decrease health and update UI
  (bind _output_get (set `self.cryoPodHealth` (- (`self.cryoPodHealth`) damage)))
  (`self.UpdateHealthBarUI` _output_get)
  (bind _asgm_space_bus (cast `/Game/Blueprints/GameModes/GM_SpaceBus` (`GameplayStatics.GetGameMode`)))
  (bind _output_get_2 (set `self.cachedGamemode` _asgm_space_bus))
  (bind _cryopodinlead (`/Game/UI/WidgetBlueprints/WBP_Leaderboard.updateLeaderboard` (`/Game/Blueprints/GameModes/GM_SpaceBus.leaderboardWidget` _asgm_space_bus) (`self.allCryopods`)))
  (set `/Game/Blueprints/GameModes/GM_SpaceBus.leadingPlayer` _cryopodinlead _output_get_2)
  (if (< (`self.cryoPodHealth`) 50.0)
    (`StaticMeshComponent.SetStaticMesh` (`self.Pod`) "/Game/3DModellingAssets/TaskModels/Cryopod/partial_destroy.partial_destroy")
    ; Destroy Player if health reaches zero
    (if (<= (`self.cryoPodHealth`) 0.0)
      (`/Engine/EditorBlueprintResources/StandardMacros.IsValid` _owningplayer
        (:`Is Valid`
          (`NiagaraFunctionLibrary.SpawnSystemAtLocation` "/Game/VFX/Niagara/NS_CharacterDeath.NS_CharacterDeath" (`SceneComponent.K2_GetComponentLocation` (`Character.Mesh` _owningplayer))))
        (:`Is Not Valid`
          _))
      (`self.K2_DestroyActor` _owningplayer)
      (`self.OnPseudoDestroyed`)
      (`self.destroyCryopodAndCheckIfAnyOtherRemain`))))

(fn `destroyCryopodAndCheckIfAnyOtherRemain`
  (bind _cachedgamemode (`self.cachedGamemode`))
  (for _array_element (`self.allCryopods`)
    (`/Engine/EditorBlueprintResources/StandardMacros.IsValid` _array_element
      (:`Is Valid`
        (if (> (`/Game/Blueprints/LevelBlueprints/BP_Cryopod.cryoPodHealth` _array_element) 0.0)
          (`/Engine/EditorBlueprintResources/StandardMacros.IncrementInt` (`self.alivePlayers`))))))
  (if (>= (`self.alivePlayers`) 2)
    (set `self.alivePlayers` 0)
    (`NiagaraFunctionLibrary.SpawnSystemAtLocation` "/Game/VFX/Niagara/NS_CharacterDeath.NS_CharacterDeath" (`SceneComponent.K2_GetComponentLocation` (`self.Pod`)))
    (`StaticMeshComponent.SetStaticMesh` (`self.Pod`) "/Game/3DModellingAssets/TaskModels/Cryopod/destroyed.destroyed")
    (`FMODBlueprintStatics.SetGlobalParameterByName` (`self.playerTrackName`) 1.0)
    (elif (not (`/Game/Blueprints/GameModes/GM_SpaceBus.isGameOver?` _cachedgamemode))
      (`/Game/Blueprints/GameModes/GM_SpaceBus.ShowEndScreen` _cachedgamemode false))))

(fn `rotateWidgetTowardsCamera`
  (params (`Widget Component` :type "WidgetComponent Object Reference"))
  (bind (_returnvalue_roll _returnvalue_pitch) (`KismetMathLibrary.BreakRotator` (`KismetMathLibrary.FindLookAtRotation` (`SceneComponent.K2_GetComponentLocation` `Widget Component`) (`SceneComponent.K2_GetComponentLocation` (`PlayerCameraManager.TransformComponent` (`UserWidget.GetOwningPlayerCameraManager` (`WidgetComponent.GetUserWidgetObject` `Widget Component`)))))))
  (`SceneComponent.K2_SetWorldRotation` `Widget Component` (`KismetMathLibrary.MakeRotator` (+ _returnvalue_roll 180.0) (+ _returnvalue_pitch 90.0)) false false))

(fn `UpdateHealthBarUI`
  (params (InputPin :type "Float (double-precision)"))
  (bind _aswbp_cryopod_health (cast `/Game/UI/WidgetBlueprints/WBP_CryopodHealth` (`WidgetComponent.GetUserWidgetObject` (`self.Widget`))))
  (`ProgressBar.SetPercent` (`/Game/UI/WidgetBlueprints/WBP_CryopodHealth.ProgressBar` _aswbp_cryopod_health) (/ InputPin (`self.initialCryoPodHealth`))))

(fn `UserConstructionScript`
  (`PrimitiveComponent.SetMaterial` (`self.Pod`) 0 (`self.podShellMaterial`))
  (`PrimitiveComponent.SetMaterial` (`self.Base`) 1 (`self.baseMaterial`)))