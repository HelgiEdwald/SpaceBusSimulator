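; BP_DoorSwitch is a lever the player can use to open a linked door, which closes again automatically after a short timer.
; Box overlaps register the switch on BP_ThirdPersonCharacter and toggle a button prompt widget, which is rotated every tick using a look-at toward the camera.
; Interact swaps the lever mesh, hides the prompt and opens DoorToOpen; the timer event reverses this, restoring the prompt if the player still overlaps.
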(event `self.ReceiveBeginPlay`
  (`self.setButtonImage` (`self.buttonImage`) (`self.ButtonPromptWidgetComponent`)))

(event `self.ReceiveTick`
  (params (DeltaSeconds :type "Float (single-precision)"))
  (`self.rotateWidgetTowardsCamera` (`self.ButtonPromptWidgetComponent`)))

(event `self.Interact`
  (if (`self.playerOverlapping`)
    (`StaticMeshComponent.SetStaticMesh` (`self.DoorSwitchMesh`) "/Game/Blueprints/LevelBlueprints/SM_DoorLevelOpen.SM_DoorLevelOpen")
    (`KismetSystemLibrary.K2_SetTimerDelegate` (delegate `Re-enable Switch`) 5.0)
    (set `self.doorOpen` true)
    (`SceneComponent.SetHiddenInGame` (`self.ButtonPromptWidgetComponent`) true false)
    (`/Game/TemplateStuff/LevelPrototyping/Interactable/Door/BP_DoorFrame.Open Door` (`self.DoorToOpen`))))

(event `Re-enable Switch`
  (`StaticMeshComponent.SetStaticMesh` (`self.DoorSwitchMesh`) "/Game/Blueprints/LevelBlueprints/SM_DoorLeverClosed.SM_DoorLeverClosed")
  (set `self.doorOpen` false)
  (`/Game/TemplateStuff/LevelPrototyping/Interactable/Door/BP_DoorFrame.Close Door` (`self.DoorToOpen`))
  (if (`self.playerOverlapping`)
    (`SceneComponent.SetHiddenInGame` (`self.ButtonPromptWidgetComponent`) false false)))

(event `self.Box.OnComponentBeginOverlap`
  (params (OverlappedComponent :type "PrimitiveComponent Object Reference") (OtherActor :type "Actor Object Reference") (OtherComp :type "PrimitiveComponent Object Reference") (OtherBodyIndex :type Integer) (bFromSweep :type Boolean) (SweepResult :type "HitResult Structure (by ref)"))
  (if (not (`/Game/TemplateStuff/LevelPrototyping/Interactable/Door/BP_DoorFrame.doorIsOpen` (`self.DoorToOpen`)))
    (if (not (`self.doorOpen`))
      (if (not (`self.playerOverlapping`))
        ; Check if overlapped actor is a player
        (if (`self.ActorHasTag` OtherActor "Player")
          (bind _asbp_third_person_character (cast `/Game/Blueprints/Characters/BP_ThirdPersonCharacter` OtherActor))
          (set `/Game/Blueprints/Characters/BP_ThirdPersonCharacter.overlappedDoorSwitch` self _asbp_third_person_character)
          (set `self.playerOverlapping` true)
          (`SceneComponent.SetHiddenInGame` (`self.ButtonPromptWidgetComponent`) false false))))))

(event `self.Box.OnComponentEndOverlap`
  (params (OverlappedComponent :type "PrimitiveComponent Object Reference") (OtherActor :type "Actor Object Reference") (OtherComp :type "PrimitiveComponent Object Reference") (OtherBodyIndex :type Integer))
  (if (`self.playerOverlapping`)
    ; Check if overlapped actor is a player
    (if (`self.ActorHasTag` OtherActor "Player")
      (bind _asbp_third_person_character (cast `/Game/Blueprints/Characters/BP_ThirdPersonCharacter` OtherActor))
      (set `/Game/Blueprints/Characters/BP_ThirdPersonCharacter.overlappedDoorSwitch` null _asbp_third_person_character)
      (set `self.playerOverlapping` false)
      (`SceneComponent.SetHiddenInGame` (`self.ButtonPromptWidgetComponent`) true false))))

(fn `enableActor`
  (params (Enable :type Boolean))
  (`self.SetActorHiddenInGame` (not Enable))
  (`self.SetActorEnableCollision` Enable))

(fn `rotateWidgetTowardsCamera`
  (params (`Widget Component` :type "WidgetComponent Object Reference"))
  (bind (_returnvalue_roll _returnvalue_pitch) (`KismetMathLibrary.BreakRotator` (`KismetMathLibrary.FindLookAtRotation` (`SceneComponent.K2_GetComponentLocation` `Widget Component`) (`SceneComponent.K2_GetComponentLocation` (`PlayerCameraManager.TransformComponent` (`UserWidget.GetOwningPlayerCameraManager` (`WidgetComponent.GetUserWidgetObject` `Widget Component`)))))))
  (`SceneComponent.K2_SetWorldRotation` `Widget Component` (`KismetMathLibrary.MakeRotator` (+ _returnvalue_roll 180.0) (+ _returnvalue_pitch 90.0)) false false))

(fn `setButtonImage`
  (params (textureToUse :type "Texture2D Object Reference") (widgetComponent :type "WidgetComponent Object Reference"))
  (bind _aswbp_button_prompt (cast `/Game/UI/WidgetBlueprints/WBP_ButtonPrompt` (`WidgetComponent.GetUserWidgetObject` widgetComponent)))
  (set `/Game/UI/WidgetBlueprints/WBP_ButtonPrompt.buttonTexture` textureToUse _aswbp_button_prompt))

(fn `UserConstructionScript`)