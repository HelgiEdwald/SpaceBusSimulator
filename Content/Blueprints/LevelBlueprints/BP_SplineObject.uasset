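; BP_SplineObject is an actor that moves a configurable mesh along the spline of a referenced SplineToFollow actor when play begins.
; The construction script applies ObjectMesh to the static mesh component.
; A timeline, with play rate set to the inverse of TimeToComplete, lerps distance over the spline's length.
; Each update sets the actor's world location and rotation from the spline at that distance.
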(event `self.ReceiveBeginPlay`
  (`self.Move Object`))

(event `Move Object`
  (bind _spline (`/Game/Blueprints/LevelBlueprints/BP_SplinePath.Spline` (`self.splineToFollow`)))
  (`TimelineComponent.SetPlayRate` (`self.T_Move`) (/ 1.0 (`self.timeToComplete`)))
  (bind (_direction _movetrack) (`Timeline|T_Move`)
    (:`Update`
      (bind _returnvalue (`KismetMathLibrary.Lerp` 0.0 (`SplineComponent.GetSplineLength` _spline) _movetrack))
      (`self.K2_SetActorLocationAndRotation` (`SplineComponent.GetLocationAtDistanceAlongSpline` _spline _returnvalue "World") (`SplineComponent.GetRotationAtDistanceAlongSpline` _spline _returnvalue "World")))))

(fn `UserConstructionScript`
  (`StaticMeshComponent.SetStaticMesh` (`self.StaticMesh`) (`self.objectMesh`)))