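; BP_GameAudio is an audio Blueprint that plays game audio through an FMOD audio component and silences it when the game ends.
; On BeginPlay it waits one tick, applies its Volume to the FMOD component, then binds StopPlayingMusic to the GM_SpaceBus game mode's OnGameEnded event.
; A helper function casts the current game mode to GM_SpaceBus and stores it before returning it.
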(event `self.ReceiveBeginPlay`
  (`KismetSystemLibrary.DelayUntilNextTick`)
  (`FMODAudioComponent.SetVolume` (`self.FMODAudio`) (`self.Volume`))
  (bind _cachedgamemode (`self.GetAndCacheGM_SpaceBus`))
  (add `/Game/Blueprints/GameModes/GM_SpaceBus.On Game Ended` _cachedgamemode (delegate `Stop Playing Music`)))

(event `Stop Playing Music`
  (`FMODAudioComponent.Stop` (`self.FMODAudio`)))

(fn `GetAndCacheGM_SpaceBus`
  (returns (CachedGameMode :type "/Game/Blueprints/GameModes/GM_SpaceBus Object Reference"))
  (bind _asgm_space_bus (cast `/Game/Blueprints/GameModes/GM_SpaceBus` (`GameplayStatics.GetGameMode`)))
  (bind _output_get (set `self.cachedGameMode` _asgm_space_bus))
  (return _output_get))

(fn `UserConstructionScript`)