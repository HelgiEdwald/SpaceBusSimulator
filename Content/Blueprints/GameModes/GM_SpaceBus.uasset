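; Game mode for SpaceBus that runs a timed round, from pre-game countdown to end screen.
; BeginPlay creates the cryopod leaderboard, countdown and HUD widgets, then starts looping timers for the countdown and round clock.
; Countdown end signals game start; round timeout pauses the game, shows LeadingPlayer as winner and signals game end.
; Another timer raises FMOD's global music intensity parameter every minute, caching the music event instance.
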(event `self.ReceiveBeginPlay`
  ; Event Begin Play
  (`self.createLeaderboardWidget`)
  ;; Display and update countdown until game begins
  (`self.createCountdownWidget`)
  (bind _returnvalue (`KismetSystemLibrary.K2_SetTimerDelegate` (delegate `Take Countdown`) 1.0 true))
  (`WidgetBlueprintLibrary.SetInputMode_GameOnly` (`GameplayStatics.GetPlayerController` 0))
  (bind _outactors (`GameplayStatics.GetAllActorsOfClass` "/Game/Blueprints/Tasks/BP_RecurringTask.BP_RecurringTask_C"))
  (set `self.MaxScore` (`KismetArrayLibrary.Array_Length` _outactors))
  ;; Create UI WIdget and Update
  (bind _returnvalue_2 (`|CreateWidget` "/Game/UI/WidgetBlueprints/WBP_UI.WBP_UI_C"))
  (bind _output_get (set `self.UserInterface` _returnvalue_2))
  (`UserWidget.AddToViewport` _output_get 0)
  (`self.updateUIElements` _output_get)
  ;; Set a looping timer to manually track time left of the game, end the game when time remaining is zero
  (`KismetSystemLibrary.K2_SetTimerDelegate` (delegate `DecreaseCount`) 1.0 true)
  ;; Update Intensity of Music every 60 seconds with FMOD parameters
  (`KismetSystemLibrary.K2_SetTimerDelegate` (delegate `Music Intensity Increased`) 60.0 true))

(event `Take Countdown`
  ; Event Begin Play
  ;; Display and update countdown until game begins
  (bind _result (`/Engine/EditorBlueprintResources/StandardMacros.DecrementInt` (`self.Countdown Time`))
    (:`  `
      (`/Game/UI/WidgetBlueprints/WBP_Countdown.UpdateText` (`self.Countdown WIdget`) _result)
      (if (<= (`self.Countdown Time`) 0)
        (`Widget.RemoveFromParent` (`self.Countdown WIdget`))
        (`KismetSystemLibrary.K2_ClearAndInvalidateTimerHandle` (stale `self.ReceiveBeginPlay` _returnvalue))
        (set `self.gameStarted` true)
        (`self.On Game Started`)))))

(event `Music Intensity Increased`
  ; Event Begin Play
  ;; Update Intensity of Music every 60 seconds with FMOD parameters
  ;;; Find instance of music in game and cache it, use cached instance of music next time event is called
  (bind _returnvalue (`FMODBlueprintStatics.EventInstanceIsValid` (`self.gameMusicEventInstance`)))
  (if (not _returnvalue)
    (bind _returnvalue_2 (`FMODBlueprintStatics.FindEventInstances` "/Game/FMOD/Events/Music/Game_Music_-_Main_Event.Game_Music_-_Main_Event"))
    (bind _output (`|GetArrayItem` _returnvalue_2))
    (`FMODBlueprintStatics.EventInstanceIsValid` _output)
    (set `self.gameMusicEventInstance` _output))
  ;;; Increase intensity parameter value by 1
  (`FMODBlueprintStatics.GetGlobalParameterByName` "intensityLevel")
  (bind _result (`/Engine/EditorBlueprintResources/StandardMacros.IncrementFloat` (`self.musicIntensity`))
    (:`  `
      (`FMODBlueprintStatics.SetGlobalParameterByName` "intensityLevel" _result))))

(event `DecreaseCount`
  (bind _roundtime (`self.roundTime`))
  ; Event Begin Play
  ;; Set a looping timer to manually track time left of the game, end the game when time remaining is zero
  ;;; Only update time after game has started and before it ends
  (if (`self.gameStarted`)
    (if (not (`self.isGameOver?`))
      ;;; Decrement time remaining and update UI element
      (bind _result (`/Engine/EditorBlueprintResources/StandardMacros.DecrementFloat` _roundtime)
        (:`  `
          (`/Game/UI/WidgetBlueprints/WBP_UI.UpdateTime` (`self.UserInterface`) _result)
          ;;; End the game when timer remaining is zero
          (if (<= _roundtime 0)
            (`self.ShowEndScreen` false)
            (`self.On Game Ended`)))))))

(event `ShowEndScreen`
  (params (`LostGame?` :type Boolean))
  ; Show end screen and display name of player with the most amount of cryopod health left
  (set `self.isGameOver?` true)
  (bind _returnvalue (`|CreateWidget` "/Game/UI/WidgetBlueprints/WBP_EndScreen.WBP_EndScreen_C" (`GameplayStatics.GetPlayerController` 0) `LostGame?`))
  (`UserWidget.AddToViewport` _returnvalue 0)
  (`/Game/UI/WidgetBlueprints/WBP_EndScreen.SetWinnerText` _returnvalue (`/Game/Blueprints/LevelBlueprints/BP_Cryopod.playerName` (`self.leadingPlayer`)))
  (`WidgetBlueprintLibrary.SetInputMode_GameAndUIEx` (`GameplayStatics.GetPlayerController` 0) _returnvalue "LockAlways" false)
  (`GameplayStatics.SetGamePaused` true))

(event `self.ReceiveTick`
  (params (DeltaSeconds :type "Float (single-precision)"))
  (`/Game/UI/WidgetBlueprints/WBP_UI.UpdateScore` (`self.UserInterface`) 0 (`self.tasksInLevel`))
  (`self.SetNumberOfTasksInLevel`))

(fn `createCountdownWidget`
  (bind _returnvalue (`|CreateWidget` "/Game/UI/WidgetBlueprints/WBP_Countdown.WBP_Countdown_C"))
  (bind _output_get (set `self.Countdown WIdget` _returnvalue))
  (`UserWidget.AddToViewport` _output_get 0)
  (`/Game/UI/WidgetBlueprints/WBP_Countdown.UpdateText` _output_get (`self.Countdown Time`)))

(fn `createLeaderboardWidget`
  (bind _returnvalue (`|CreateWidget` "/Game/UI/WidgetBlueprints/WBP_Leaderboard.WBP_Leaderboard_C"))
  (bind _output_get (set `self.leaderboardWidget` _returnvalue))
  (`UserWidget.AddToViewport` _output_get 0)
  (bind _outactors (`GameplayStatics.GetAllActorsOfClass` "/Game/Blueprints/LevelBlueprints/BP_Cryopod.BP_Cryopod_C"))
  (`/Game/UI/WidgetBlueprints/WBP_Leaderboard.updateLeaderboard` _returnvalue _outactors))

(fn `determineRating`
  (returns (rating :type String))
  (return (select `int` (`KismetMathLibrary.FTrunc` (`KismetMathLibrary.FClamp` (/ (`self.shipHealth`) 200.0) 0.0 4.99)) :`0` "F" :`1` "C" :`2` "B" :`3` "A" :`4` "S")))

(fn `SetGameInputForAllPlayers`
  (bind _outactors (`GameplayStatics.GetAllActorsOfClass` "/Script/Engine.PlayerController"))
  (for _array_element _outactors
    (`WidgetBlueprintLibrary.SetInputMode_GameOnly` _array_element)))

(fn `SetNumberOfTasksInLevel`
  (bind _outactors (`GameplayStatics.GetAllActorsOfClass` "/Game/Blueprints/Tasks/BP_RecurringTask.BP_RecurringTask_C"))
  (set `self.tasksInLevel` (`KismetArrayLibrary.Array_Length` _outactors)))

(fn `SetUIInputForAllPlayers`
  (bind _outactors (`GameplayStatics.GetAllActorsOfClass` "/Script/Engine.PlayerController"))
  (for _array_element _outactors
    (`WidgetBlueprintLibrary.SetInputMode_UIOnlyEx` _array_element (`self.UserInterface`))))

(fn `setViewToCameraActor`
  (bind _outactors (`GameplayStatics.GetAllActorsOfClass` "/Script/Engine.CameraActor"))
  (`PlayerController.SetViewTargetWithBlend` (`GameplayStatics.GetPlayerController` 0) (`|GetArrayItem` _outactors) 0.0 "VTBlend_Linear" 0.0 false))

(fn `updateUIElements`
  (params (`UI Widget` :type "/Game/UI/WidgetBlueprints/WBP_UI Object Reference"))
  (`/Game/UI/WidgetBlueprints/WBP_UI.UpdateScore` `UI Widget` 0 (`self.tasksInLevel`))
  (`/Game/UI/WidgetBlueprints/WBP_UI.UpdateTime` `UI Widget` (`self.roundTime`))
  (`/Game/UI/WidgetBlueprints/WBP_UI.UpdateShipHealth` `UI Widget` (`self.startingShipHealth`)))

(fn `UserConstructionScript`)