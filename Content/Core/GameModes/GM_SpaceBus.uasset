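; Game mode for SpaceBus that runs a timed round from countdown to end screen.
; BeginPlay switches to a level camera, creates the leaderboard, countdown and HUD widgets, and starts looping one-second timers that fire game start and end dispatchers.
; Tick recounts recurring task actors for the HUD, with current score fixed at zero.
; The end screen shows the leading player and a ship-health letter grade, then switches players to UI input.
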(event `self.ReceiveBeginPlay`
  (`self.createLeaderboardWidget`)
  ; Event Begin Play
  ;; Countdown
  (`self.createCountdownWidget`)
  (bind _returnvalue (`KismetSystemLibrary.K2_SetTimerDelegate` (delegate `Take Countdown`) 1.0 true))
  (`self.setViewToCameraActor`)
  ;; Create UI WIdget and Update Score
  (bind _outactors (`GameplayStatics.GetAllActorsOfClass` "/Game/Core/Tasks/BP_RecurringTaskSpawner.BP_RecurringTaskSpawner_C"))
  (set `self.taskSpawnersInGame` (`KismetArrayLibrary.Array_Length` _outactors))
  (`WidgetBlueprintLibrary.SetInputMode_GameOnly` (`GameplayStatics.GetPlayerController` 0))
  (bind _outactors_2 (`GameplayStatics.GetAllActorsOfClass` "/Game/Core/Tasks/BP_RecurringTask.BP_RecurringTask_C"))
  (set `self.MaxScore` (`KismetArrayLibrary.Array_Length` _outactors_2))
  (bind _returnvalue_2 (`|CreateWidget` "/Game/UI/WBP_UI.WBP_UI_C"))
  (bind _output_get (set `self.UserInterface` _returnvalue_2))
  (`UserWidget.AddToViewport` _output_get 0)
  (`self.updateUIElements` _output_get)
  ;; Timer that decreases by 1 second and shows end screen when it reaches zero
  (`KismetSystemLibrary.K2_SetTimerDelegate` (delegate `DecreaseCount`) 1.0 true))

(event `Take Countdown`
  ; Event Begin Play
  ;; Countdown
  (bind _result (`/Engine/EditorBlueprintResources/StandardMacros.DecrementInt` (`self.Countdown Time`))
    (:`  `
      (`/Game/UI/WBP_Countdown.UpdateText` (`self.Countdown WIdget`) _result)
      (if (<= (`self.Countdown Time`) 0)
        (`Widget.RemoveFromParent` (`self.Countdown WIdget`))
        (`KismetSystemLibrary.K2_ClearAndInvalidateTimerHandle` (stale `self.ReceiveBeginPlay` _returnvalue))
        (set `self.gameStarted` true)
        (`self.On Game Started`)))))

(event `DecreaseCount`
  (bind _roundtime (`self.roundTime`))
  ; Event Begin Play
  ;; Timer that decreases by 1 second and shows end screen when it reaches zero
  (if (`self.gameStarted`)
    (if (not (`self.isGameOver?`))
      (bind _result (`/Engine/EditorBlueprintResources/StandardMacros.DecrementFloat` _roundtime)
        (:`  `
          (`/Game/UI/WBP_UI.UpdateTime` (`self.UserInterface`) _result)
          (if (<= _roundtime 0)
            (`self.ShowEndScreen` false)
            (`self.On Game Ended`)))))))

(event `self.ReceiveTick`
  (params (DeltaSeconds :type "Float (single-precision)"))
  ; Event Tick
  (`/Game/UI/WBP_UI.UpdateScore` (`self.UserInterface`) 0 (`self.tasksInLevel`))
  (`self.SetNumberOfTasksInLevel`))

(event `ShowEndScreen`
  (params (`LostGame?` :type Boolean))
  (bind _returnvalue (`GameplayStatics.GetPlayerController` 0))
  ; Show End Screen Event with Game Outcome as a Parameter
  (set `self.isGameOver?` true)
  (bind _returnvalue_2 (`|CreateWidget` "/Game/UI/WBP_EndScreen.WBP_EndScreen_C" null `LostGame?`))
  (`UserWidget.AddToViewport` _returnvalue_2 0)
  (`/Game/UI/WBP_EndScreen.SetWinnerText` _returnvalue_2 (`/Game/Core/BP_Cryopod.playerName` (`self.leadingPlayer`)))
  (bind _rating (`self.determineRating`))
  (`/Game/UI/WBP_EndScreen.Add Rating` _returnvalue_2 _rating)
  (`WidgetBlueprintLibrary.SetInputMode_GameAndUIEx` _returnvalue _returnvalue_2 "LockAlways" false)
  (set `PlayerController.bShowMouseCursor` true _returnvalue)
  (`KismetSystemLibrary.Delay` 0.2)
  (`self.SetUIInputForAllPlayers`)
  (`Widget.SetFocus` (`/Game/UI/WBP_EndScreen.RestartButton` _returnvalue_2)))

(fn `createCountdownWidget`
  (bind _returnvalue (`|CreateWidget` "/Game/UI/WBP_Countdown.WBP_Countdown_C"))
  (bind _output_get (set `self.Countdown WIdget` _returnvalue))
  (`UserWidget.AddToViewport` _output_get 0)
  (`/Game/UI/WBP_Countdown.UpdateText` _output_get (`self.Countdown Time`)))

(fn `createLeaderboardWidget`
  (bind _returnvalue (`|CreateWidget` "/Game/UI/WBP_Leaderboard.WBP_Leaderboard_C"))
  (bind _output_get (set `self.leaderboardWidget` _returnvalue))
  (`UserWidget.AddToViewport` _output_get 0)
  (bind _outactors (`GameplayStatics.GetAllActorsOfClass` "/Game/Core/BP_Cryopod.BP_Cryopod_C"))
  (`/Game/UI/WBP_Leaderboard.updateLeaderboard` _returnvalue _outactors))

(fn `determineRating`
  (returns (rating :type String))
  (return (select `int` (`KismetMathLibrary.FTrunc` (`KismetMathLibrary.FClamp` (/ (`self.shipHealth`) 200.0) 0.0 4.99)) :`0` "F" :`1` "C" :`2` "B" :`3` "A" :`4` "S")))

(fn `SetGameInputForAllPlayers`
  (bind _outactors (`GameplayStatics.GetAllActorsOfClass` "/Script/Engine.PlayerController"))
  (for _array_element _outactors
    (`KismetSystemLibrary.PrintString` (`KismetSystemLibrary.GetDisplayName` _array_element))
    (`WidgetBlueprintLibrary.SetInputMode_GameOnly` _array_element)))

(fn `SetNumberOfTasksInLevel`
  (bind _outactors (`GameplayStatics.GetAllActorsOfClass` "/Game/Core/Tasks/BP_RecurringTask.BP_RecurringTask_C"))
  (set `self.tasksInLevel` (`KismetArrayLibrary.Array_Length` _outactors)))

(fn `SetUIInputForAllPlayers`
  (bind _outactors (`GameplayStatics.GetAllActorsOfClass` "/Script/Engine.PlayerController"))
  (for _array_element _outactors
    (`WidgetBlueprintLibrary.SetInputMode_UIOnlyEx` _array_element (`self.UserInterface`))))

(fn `setViewToCameraActor`
  (bind _outactors (`GameplayStatics.GetAllActorsOfClass` "/Script/Engine.CameraActor"))
  (`PlayerController.SetViewTargetWithBlend` (`GameplayStatics.GetPlayerController` 0) (`|GetArrayItem` _outactors) 0.0 "VTBlend_Linear" 0.0 false))

(fn `updateUIElements`
  (params (`UI Widget` :type "/Game/UI/WBP_UI Object Reference"))
  (`/Game/UI/WBP_UI.UpdateScore` `UI Widget` 0 (`self.tasksInLevel`))
  (`/Game/UI/WBP_UI.UpdateTime` `UI Widget` (`self.roundTime`))
  (`/Game/UI/WBP_UI.UpdateShipHealth` `UI Widget` (`self.startingShipHealth`)))

(fn `UserConstructionScript`)