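; BP_Leaderboard is a leaderboard Blueprint that ranks cryopod actors by their health, highest first.
; SortCryoBodArray runs an insertion sort, casting each element to BP_Cryopod and scanning the sorted list backward for its slot by CryoPodHealth.
; The inline comment about distance to the player does not match this health comparison.
; The event graph, construction script and SortArray function are empty.
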(fn `sortArray`)

(fn `sortCryoBodArray`
  (params (arrayToSort :type "Array of /Game/Core/BP_Cryopod Object Reference"))
  (returns (`Sorted By Distance` :type "Array of Actor Object Reference"))
  (locals (`Sorted Array` :type "Array of Actor Object Reference") (`Current Actor` :type "Actor Object Reference") (`Insert Index` :type Integer) (`Working Array` :type "Array of Actor Object Reference") (`Current Health` :type "Float (single-precision)"))
  (bind _output_get (set `local.Working Array` arrayToSort))
  (for _array_element _output_get
    ;[1 1 1] Get compartive value
    (bind _asbp_cryopod (cast `/Game/Core/BP_Cryopod` _array_element))
    (set `local.Current Actor` _array_element)
    (set `local.Current Health` (`/Game/Core/BP_Cryopod.cryoPodHealth` _asbp_cryopod))
    ;[1 1 1] Add to end by default
    (set `local.Insert Index` (`KismetArrayLibrary.Array_Length` (`local.Sorted Array`)))
    ;[1 1 1] Loop backward through already sorted list. If a new actor is closer to the player, move it down the list
    (bind (_arrayindex _arrayelement) (`/Engine/EditorBlueprintResources/StandardMacros.ReverseForEachLoop` (`local.Sorted Array`))
      (:`LoopBody`
        (bind _asbp_cryopod_2 (cast `/Game/Core/BP_Cryopod` _arrayelement))
        (if (< (`/Game/Core/BP_Cryopod.cryoPodHealth` _asbp_cryopod_2) (`local.Current Health`))
          (set `local.Insert Index` _arrayindex)))
      (:`Completed`
        (`KismetArrayLibrary.Array_Insert` (`local.Sorted Array`) (`local.Current Actor`) (`local.Insert Index`)))))
  (return (`local.Sorted Array`)))

(fn `UserConstructionScript`)