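; BP_SlimeTask is a task actor for slime that the player clears by interacting while holding a broom.
; On Interact, it searches overlapping BP_ThirdPersonCharacter actors for one tagged Player whose HasBroom flag is set.
; When one is found, it sets PlayerHasItem, plays the task-complete sound in 2D and destroys itself.
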(event `self.ReceiveBeginPlay`
  (`parent.ReceiveBeginPlay`))

(event `/Game/Core/BPI_UseItem.Interact`
  ;[0 0 1 0.5] Play Sound and Destroy Self Upon Interact Message
  (for _array_element (`self.GetOverlappingActors` "/Game/Core/BP_ThirdPersonCharacter.BP_ThirdPersonCharacter_C")
    (if (`self.ActorHasTag` _array_element "Player")
      (if (`/Game/Core/BP_ThirdPersonCharacter.HasBroom` _array_element)
        (set `self.playerHasItem` true)
        (break))))
  (if (`self.playerHasItem`)
    (`GameplayStatics.SpawnSound2D` "/Game/Audio/In-House/SW_TaskComplete.SW_TaskComplete" 1.0 1.0 0.0 null)
    (`self.K2_DestroyActor`)))

(fn `UserConstructionScript`
  (`parent.UserConstructionScript`))