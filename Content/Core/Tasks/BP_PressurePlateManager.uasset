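; BP_PressurePlateManager is an alert task that completes when every pressure plate in the level is active at the same time.
; On BeginPlay it gathers all BP_PressurePlate actors, enables them after a short delay and binds to their activation events.
; Each activation rechecks all plates; when all are active it calls AlertTaskCompleted, turns them green, flags them completed and destroys them after a pause.
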(event `self.ReceiveBeginPlay`
  ; Inherit Alert Task Logic
  (`parent.ReceiveBeginPlay`)
  (bind _outactors (`GameplayStatics.GetAllActorsOfClass` "/Game/Core/Tasks/BP_PressurePlate.BP_PressurePlate_C"))
  (bind _output_get (set `self.pressurePlateArray` _outactors))
  (set `self.numPressurePlates` (`KismetArrayLibrary.Array_Length` _outactors))
  (`KismetSystemLibrary.Delay` 0.2)
  (for _array_element _output_get
    (`/Game/Core/Tasks/BP_PressurePlate.enableActor` _array_element true))
  (for _array_element_2 (`self.pressurePlateArray`)
    (add `/Game/Core/Tasks/BP_PressurePlate.OnPlateActivated` _array_element_2 (delegate `CheckAllPlates`))))

(event `CheckAllPlates`
  (bind _pressureplatearray (`self.pressurePlateArray`))
  (for _array_element (`self.pressurePlateArray`)
    (if (`/Game/Core/Tasks/BP_PressurePlate.pressurePlateActivated` _array_element)
      (set `self.atLeastOnePlateInactive` false)
      (else
        (set `self.atLeastOnePlateInactive` true)
        (break))))
  (if (not (`self.atLeastOnePlateInactive`))
    (`self.AlertTaskCompleted`)
    (for _array_element_2 _pressureplatearray
      (`PrimitiveComponent.SetMaterial` (`/Game/Core/Tasks/BP_PressurePlate.PressurePlateStaticMesh` _array_element_2) 0 "/AnimationSharing/AnimSharingGreen.AnimSharingGreen")
      (set `/Game/Core/Tasks/BP_PressurePlate.taskCompleted` true _array_element_2))
    (`KismetSystemLibrary.Delay` 3.0)
    (for _array_element_3 _pressureplatearray
      (`self.K2_DestroyActor` _array_element_3))))

(fn `UserConstructionScript`
  (`parent.UserConstructionScript`))