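; BP_AlertTaskSpawner spawns an alert task actor at its root transform while the GM_SpaceBus game is not over.
; Normally it spawns once, either on game start or at a random time 50–75% through the round.
; In alternate mode, a looping 30-second timer spawns instead, then changes a light switch manager class to pressure plate manager.
; Any other class gets replaced by the failed cast result.
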(event `Spawn Alert Task`
  (bind _actor_to_spawn (`self.Actor to Spawn`))
  (if (not (`/Game/Core/GameModes/GM_SpaceBus.isGameOver?` (`self.cachedGameMode`)))
    (if (`KismetSystemLibrary.IsValidClass` _actor_to_spawn)
      (`|SpawnActorFromClass` _actor_to_spawn (`SceneComponent.K2_GetComponentToWorld` (`self.DefaultSceneRoot`)) "Undefined" "MultiplyWithRoot" null null)
      (bind _asbp_light_switch_manager (castclass `/Game/Core/Tasks/BP_LightSwitchManager` (`self.Actor to Spawn`))
        (:`then`
          (set `self.Actor to Spawn` "/Game/Core/Tasks/BP_PressurePlateManager.BP_PressurePlateManager_C"))
        (:`CastFailed`
          (set `self.Actor to Spawn` _asbp_light_switch_manager))))))

(event `self.ReceiveBeginPlay`
  ; Event BeginPlay
  (bind _cachedgamemode (`self.GetAndCacheGM_SpaceBus`))
  (if (`self.alternateGameMode`)
    (`KismetSystemLibrary.K2_SetTimerDelegate` (delegate `Spawn Alert Task`) 30.0 true)
    (elif (`self.spawnInSecondHalfOfRound`)
      (bind _roundtime (`/Game/Core/GameModes/GM_SpaceBus.roundTime` _cachedgamemode))
      (`KismetSystemLibrary.K2_SetTimerDelegate` (delegate `Spawn Actor at Location`) (`KismetMathLibrary.RandomFloatInRange` (* _roundtime 0.5) (* _roundtime 0.75)))
      (else
        (add `/Game/Core/GameModes/GM_SpaceBus.On Game Started` (`self.cachedGameMode`) (delegate `Spawn Actor at Location`))))))

(event `Spawn Actor at Location`
  (bind _actor_to_spawn (`self.Actor to Spawn`))
  ; Event BeginPlay
  ;; Check if game over
  (if (not (`/Game/Core/GameModes/GM_SpaceBus.isGameOver?` (`self.cachedGameMode`)))
    (if (`KismetSystemLibrary.IsValidClass` _actor_to_spawn)
      (`|SpawnActorFromClass` _actor_to_spawn (`SceneComponent.K2_GetComponentToWorld` (`self.DefaultSceneRoot`)) "Undefined" "MultiplyWithRoot" null null))))

(fn `GetAndCacheGM_SpaceBus`
  (returns (CachedGameMode :type "/Game/Core/GameModes/GM_SpaceBus Object Reference"))
  (bind _asgm_space_bus (cast `/Game/Core/GameModes/GM_SpaceBus` (`GameplayStatics.GetGameMode`)))
  (bind _output_get (set `self.cachedGameMode` _asgm_space_bus))
  (return _output_get))

(fn `UserConstructionScript`)