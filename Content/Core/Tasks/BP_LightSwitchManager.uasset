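; Task manager for a light switch task that darkens the level's sun until every BP_LightSwitch is turned on.
; On BeginPlay it finds the BP_Sun by the "Sun" tag, calls GoDark, then enables all switches and binds their activation events.
; Each activation rechecks all switches; full activation completes the task, calls GoLight and destroys the switches after a delay.
; Task failure destroys the switches immediately.
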(event `self.ReceiveBeginPlay`
  (`parent.ReceiveBeginPlay`)
  (bind _outactors (`GameplayStatics.GetAllActorsWithTag` "Sun"))
  (bind _asbp_sun (cast `/Game/Core/BP_Sun` (`|GetArrayItem` _outactors)))
  (bind _output_get (set `self.As BP Sun` _asbp_sun))
  (`/Game/Core/BP_Sun.goDark` _output_get)
  (bind _outactors_2 (`GameplayStatics.GetAllActorsOfClass` "/Game/Core/Tasks/BP_LightSwitch.BP_LightSwitch_C"))
  (bind _output_get_2 (set `self.lightSwitchArray` _outactors_2))
  (set `self.numLightSwitches` (`KismetArrayLibrary.Array_Length` _outactors_2))
  (`KismetSystemLibrary.Delay` 0.2)
  (for _array_element _output_get_2
    (`/Game/Core/Tasks/BP_LightSwitch.enableActor` _array_element true))
  (for _array_element_2 (`self.lightSwitchArray`)
    (add `/Game/Core/Tasks/BP_LightSwitch.OnLightSwitchActivated` _array_element_2 (delegate `CheckAllSwitches`))
    (add `self.OnAlertTaskFailed` (delegate `DeleteParts`))))

(event `DeleteParts`
  (for _array_element (`self.lightSwitchArray`)
    (`self.K2_DestroyActor` _array_element)))

(event `CheckAllSwitches`
  (bind _lightswitcharray (`self.lightSwitchArray`))
  (for _array_element (`self.lightSwitchArray`)
    (if (`/Game/Core/Tasks/BP_LightSwitch.lightSwitchActivated` _array_element)
      (set `self.atLeast1SwitchOff` false)
      (else
        (set `self.atLeast1SwitchOff` true)
        (break))))
  (if (not (`self.atLeast1SwitchOff`))
    (`self.AlertTaskCompleted`)
    (for _array_element_2 _lightswitcharray
      (set `/Game/Core/Tasks/BP_LightSwitch.Task Completed` true _array_element_2))
    (`KismetSystemLibrary.Delay` 3.0)
    (for _array_element_3 _lightswitcharray
      (`self.K2_DestroyActor` _array_element_3))))

(fn `AlertTaskCompleted`
  (`parent.AlertTaskCompleted`)
  (`/Game/Core/BP_Sun.goLight` (`self.As BP Sun`)))

(fn `AlertTaskFailed`
  (`parent.AlertTaskFailed`))

(fn `UserConstructionScript`
  (`parent.UserConstructionScript`))