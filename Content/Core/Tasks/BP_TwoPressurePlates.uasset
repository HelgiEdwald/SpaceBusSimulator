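; Alert task actor with two pressure plates that players must hold at the same time to complete it.
; Player overlap plays audio and starts a countdown that turns that plate blue; leaving early stops both, resets it and turns it red.
; With both plates finished, they turn green, the inherited alert task completes and the actor self-destructs after a delay.
; Both plates share one timer handle, so leaving clears whichever timer was set last.
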(event `self.ReceiveBeginPlay`
  ; Inherit Alert Task Logic
  (`parent.ReceiveBeginPlay`))

(event `self.Trigger A.OnComponentBeginOverlap`
  (params (OverlappedComponent :type "PrimitiveComponent Object Reference") (OtherActor :type "Actor Object Reference") (OtherComp :type "PrimitiveComponent Object Reference") (OtherBodyIndex :type Integer) (bFromSweep :type Boolean) (SweepResult :type "HitResult Structure (by ref)"))
  ; Triggers Begin Overlap
  ;; Player Enters Trigger A
  (if (`self.ActorHasTag` OtherActor "Player")
    (`AudioComponent.Play` (`self.Audio Component for Activation`) 0.0)
    (bind _returnvalue (`KismetSystemLibrary.K2_SetTimerDelegate` (delegate `UpdateTimer`) (`self.countDownTime`)))
    (set `self.timerHandle` _returnvalue)))

(event `UpdateTimer`
  ; Triggers Begin Overlap
  ;; Player Enters Trigger A
  (set `self.pressurePlateAFinished` true)
  (`PrimitiveComponent.SetMaterial` (`self.Static Mesh A`) 0 "/Game/TemplateStuff/LevelPrototyping/Materials/MI_Solid_Blue.MI_Solid_Blue")
  ; Task Requirements Met
  (if (and (`self.pressurePlateAFinished`) (`self.pressurePlateBFinished`)) :!label _label
    (set `self.bothFinished` true)
    (`PrimitiveComponent.SetMaterial` (`self.Static Mesh A`) 0 "/AnimationSharing/AnimSharingGreen.AnimSharingGreen")
    (`PrimitiveComponent.SetMaterial` (`self.Static Mesh B`) 0 "/AnimationSharing/AnimSharingGreen.AnimSharingGreen")
    (`self.AlertTaskCompleted`)
    (set `self.taskCompleted` true)
    (`KismetSystemLibrary.Delay` 5.0)
    (`self.K2_DestroyActor`)))

(event `self.Trigger B.OnComponentBeginOverlap`
  (params (OverlappedComponent :type "PrimitiveComponent Object Reference") (OtherActor :type "Actor Object Reference") (OtherComp :type "PrimitiveComponent Object Reference") (OtherBodyIndex :type Integer) (bFromSweep :type Boolean) (SweepResult :type "HitResult Structure (by ref)"))
  ; Triggers Begin Overlap
  ;; Player Enters Trigger B
  (if (`self.ActorHasTag` OtherActor "Player")
    (`AudioComponent.Play` (`self.Audio Component for Activation`) 0.0)
    (bind _returnvalue (`KismetSystemLibrary.K2_SetTimerDelegate` (delegate `TimerB`) (`self.countDownTime`)))
    (set `self.timerHandle` _returnvalue)))

(event `TimerB`
  ; Triggers Begin Overlap
  ;; Player Enters Trigger B
  (set `self.pressurePlateBFinished` true)
  (`PrimitiveComponent.SetMaterial` (`self.Static Mesh B`) 0 "/Game/TemplateStuff/LevelPrototyping/Materials/MI_Solid_Blue.MI_Solid_Blue")
  (goto _label))

(event `self.Trigger A.OnComponentEndOverlap`
  (params (OverlappedComponent :type "PrimitiveComponent Object Reference") (OtherActor :type "Actor Object Reference") (OtherComp :type "PrimitiveComponent Object Reference") (OtherBodyIndex :type Integer))
  ; Triggers End Overlap
  ;; Player Leaves Trigger A
  (if (not (`self.taskCompleted`))
    (if (`self.ActorHasTag` OtherActor "Player")
      (`AudioComponent.Stop` (`self.Audio Component for Activation`))
      (`KismetSystemLibrary.K2_ClearAndInvalidateTimerHandle` (`self.timerHandle`))
      (set `self.pressurePlateAFinished` false)
      (`PrimitiveComponent.SetMaterial` (`self.Static Mesh A`) 0 "/AnimationSharing/AnimSharingRed.AnimSharingRed"))))

(event `self.Trigger B.OnComponentEndOverlap`
  (params (OverlappedComponent :type "PrimitiveComponent Object Reference") (OtherActor :type "Actor Object Reference") (OtherComp :type "PrimitiveComponent Object Reference") (OtherBodyIndex :type Integer))
  ; Triggers End Overlap
  ;; Player Leaves Trigger B
  (if (not (`self.taskCompleted`))
    (if (`self.ActorHasTag` OtherActor "Player")
      (`AudioComponent.Stop` (`self.Audio Component for Activation`))
      (`KismetSystemLibrary.K2_ClearAndInvalidateTimerHandle` (`self.timerHandle`))
      (set `self.pressurePlateBFinished` false)
      (`PrimitiveComponent.SetMaterial` (`self.Static Mesh B`) 0 "/AnimationSharing/AnimSharingRed.AnimSharingRed"))))

(fn `UserConstructionScript`)