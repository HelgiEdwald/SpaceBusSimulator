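; Spawn manager that places tasks through an array of spawners during a match, running only when active.
; After the GM_SpaceBus countdown, it shuffles the spawners, triggers enough for the starting task count and marks them unavailable.
; A looping timer, started at BeginPlay, reshuffles and triggers the first available spawner at each interval until the cached game mode reports game over.
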(event `self.ReceiveBeginPlay`
  ; Event Begin Play
  (if (`self.isActive`)
    (bind _cachedgamemode (`self.GetAndCacheGM_SpaceBus`))
    ;; Spawn tasks after countdown
    (`KismetSystemLibrary.K2_SetTimerDelegate` (delegate `SpawnStartingRecurringTasks`) (`KismetMathLibrary.Conv_IntToDouble` (`/Game/Core/GameModes/GM_SpaceBus.Countdown Time` _cachedgamemode)))
    ;; Check at an interval if there is an available spawner and spawn if available
    (`KismetSystemLibrary.K2_SetTimerDelegate` (delegate `Spawn New Task`) (`self.spawnNewTaskSeconds`) true false 10.0)))

(event `Spawn New Task`
  (bind _spawnerarray (`self.spawnerArray`))
  ; Event Begin Play
  ;; Check at an interval if there is an available spawner and spawn if available
  (if (not (`/Game/Core/GameModes/GM_SpaceBus.isGameOver?` (`self.cachedGameMode`)))
    (`KismetArrayLibrary.Array_Shuffle` _spawnerarray)
    (for _array_element _spawnerarray
      (bind _spawneravailable (`/Game/Core/Tasks/BP_RecurringTaskSpawner.spawnerAvailable` _array_element))
      (if _spawneravailable
        (set `self.foundAvailableSpawn` _spawneravailable)
        (`/Game/Core/Tasks/BP_RecurringTaskSpawner.Spawn Actor at Location` _array_element)
        (break)))))

(event `SpawnStartingRecurringTasks`
  (bind _spawnerarray (`self.spawnerArray`))
  ; Event Begin Play
  ;; Spawn tasks after countdown
  ;;; Shuffle array and spawn based on starting number
  (`KismetArrayLibrary.Array_Shuffle` _spawnerarray)
  (bind _result (`/Engine/EditorBlueprintResources/StandardMacros.DecrementInt` (`self.numStartingTasks`))
    (:`  `
      (for _index (range (+ _result 1))
        (bind _output (`|GetArrayItem` _spawnerarray _index))
        (`/Engine/EditorBlueprintResources/StandardMacros.IsValid` _output
          (:`Is Valid`
            (`/Game/Core/Tasks/BP_RecurringTaskSpawner.Spawn Actor at Location` _output)
            (set `/Game/Core/Tasks/BP_RecurringTaskSpawner.spawnerAvailable` false _output))
          (:`Is Not Valid`
            (`KismetSystemLibrary.PrintString` (`KismetStringLibrary.Conv_IntToString` (`KismetArrayLibrary.Array_Length` _spawnerarray)))))))))

(fn `GetAndCacheGM_SpaceBus`
  (returns (CachedGameMode :type "/Game/Core/GameModes/GM_SpaceBus Object Reference"))
  (bind _asgm_space_bus (cast `/Game/Core/GameModes/GM_SpaceBus` (`GameplayStatics.GetGameMode`)))
  (bind _output_get (set `self.cachedGameMode` _asgm_space_bus))
  (return _output_get))

(fn `UserConstructionScript`)