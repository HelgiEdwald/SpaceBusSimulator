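; BP_PooledActor is an object pool actor that is switched on and off through an InUse state.
; SetInUse stores the state and toggles collision, visibility and actor tick to match, starting inactive on BeginPlay.
; Activation restarts a TimeToLive timer that calls ReturnToPool, which deactivates the actor instead of destroying it.
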(event `self.ReceiveBeginPlay`
  (`self.SetInUse` false))

(event `SetInUse`
  (params (inUse :type Boolean))
  (set `self.inUse` inUse)
  (`self.SetActorEnableCollision` inUse)
  (`self.SetActorHiddenInGame` (not inUse))
  (`self.SetActorTickEnabled` inUse)
  (`KismetSystemLibrary.K2_ClearAndInvalidateTimerHandle` (`self.timeToLiveTimer`))
  (if inUse
    (bind _returnvalue (`KismetSystemLibrary.K2_SetTimerDelegate` (delegate `ReturnToPool`) (`self.timeToLive`)))
    (set `self.timeToLiveTimer` _returnvalue)))

(event `ReturnToPool`
  (`self.SetInUse` false))

(fn `UserConstructionScript`)