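; BP_RevolvingDoor is a spinning obstacle that knocks the player away on contact.
; Tick continuously yaws the Cylinder component at RotationSpeed, scaled by delta time.
; Hit events on four cube meshes feed BumpCharacter, which filters for the Player tag and casts to BP_ThirdPersonCharacter.
; It then launches the character horizontally away from the struck cube's origin, scaled by BumpStrength, overriding XY velocity only.
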(event `self.ReceiveTick`
  (params (DeltaSeconds :type "Float (single-precision)"))
  (`SceneComponent.K2_AddLocalRotation` (`self.Cylinder`) (`KismetMathLibrary.MakeRotator` 0.0 0.0 (* DeltaSeconds (`self.rotationSpeed`))) false false))

(event `self.Cube.OnComponentHit`
  (params (HitComponent :type "PrimitiveComponent Object Reference") (OtherActor :type "Actor Object Reference") (OtherComp :type "PrimitiveComponent Object Reference") (NormalImpulse :type "Vector Structure") (Hit :type "HitResult Structure (by ref)"))
  (`self.bumpCharacter` (`self.Cube`) OtherActor))

(event `self.Cube1.OnComponentHit`
  (params (HitComponent :type "PrimitiveComponent Object Reference") (OtherActor :type "Actor Object Reference") (OtherComp :type "PrimitiveComponent Object Reference") (NormalImpulse :type "Vector Structure") (Hit :type "HitResult Structure (by ref)"))
  (`self.bumpCharacter` (`self.Cube1`) OtherActor))

(event `self.Cube2.OnComponentHit`
  (params (HitComponent :type "PrimitiveComponent Object Reference") (OtherActor :type "Actor Object Reference") (OtherComp :type "PrimitiveComponent Object Reference") (NormalImpulse :type "Vector Structure") (Hit :type "HitResult Structure (by ref)"))
  (`self.bumpCharacter` (`self.Cube2`) OtherActor))

(event `self.Cube3.OnComponentHit`
  (params (HitComponent :type "PrimitiveComponent Object Reference") (OtherActor :type "Actor Object Reference") (OtherComp :type "PrimitiveComponent Object Reference") (NormalImpulse :type "Vector Structure") (Hit :type "HitResult Structure (by ref)"))
  (`self.bumpCharacter` (`self.Cube3`) OtherActor))

(fn `bumpCharacter`
  (params (hitMesh :type "StaticMeshComponent Object Reference") (characterHit :type "Actor Object Reference"))
  (if (`self.ActorHasTag` characterHit "Player")
    (bind _asbp_third_person_character (cast `/Game/Core/BP_ThirdPersonCharacter` characterHit))
    (bind (_returnvalue_x _returnvalue_y) (`KismetMathLibrary.BreakVector` (- (`SceneComponent.K2_GetComponentLocation` (`Character.CapsuleComponent` _asbp_third_person_character)) (`SceneComponent.K2_GetComponentLocation` hitMesh))))
    (`Character.LaunchCharacter` _asbp_third_person_character (* (`KismetMathLibrary.Normal` (`KismetMathLibrary.MakeVector` _returnvalue_x _returnvalue_y)) (`self.bumpStrength`)) true false)))

(fn `UserConstructionScript`)